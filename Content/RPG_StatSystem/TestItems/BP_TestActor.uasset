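; BP_TestActor is a test item actor in the RPG stat system that displays a text message and reacts when the player overlaps its box.
; BeginPlay caches the player as BP_ThirdPersonCharacter and sets the TextRender to DisplayMessage.
; Box overlap calls StartOverlapEffect only for that character.
; StartOverlapEffect just returns the cached character here, with no effect of its own, and end overlap does nothing.
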(event `self.ReceiveBeginPlay`
  (bind _asbp_third_person_character (cast `/Game/ThirdPerson/Blueprints/BP_ThirdPersonCharacter` (`GameplayStatics.GetPlayerCharacter` 0)))
  (set `self.Player Character` _asbp_third_person_character)
  (`TextRenderComponent.K2_SetText` (`self.TextRender`) (`self.Display Message`)))

(event `self.Box.OnComponentBeginOverlap`
  (params (OverlappedComponent :type "PrimitiveComponent Object Reference") (OtherActor :type "Actor Object Reference") (OtherComp :type "PrimitiveComponent Object Reference") (OtherBodyIndex :type Integer) (bFromSweep :type Boolean) (SweepResult :type "HitResult Structure (by ref)"))
  (if (== OtherActor (`self.Player Character`))
    (`self.Start Overlap Effect`)))

(event `self.Box.OnComponentEndOverlap`
  (params (OverlappedComponent :type "PrimitiveComponent Object Reference") (OtherActor :type "Actor Object Reference") (OtherComp :type "PrimitiveComponent Object Reference") (OtherBodyIndex :type Integer)))

(fn `Start Overlap Effect`
  (returns (Target :type "Actor Object Reference"))
  (return (`self.Player Character`)))

(fn `UserConstructionScript`)