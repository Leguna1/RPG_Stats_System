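; Inventory component that stores items and quantities in a fixed number of slots, using a map from slot index to item struct.
; Adding tops up matching stacks before filling empty slots, and drag-drop moves, merges or swaps slots.
; Using an item asks the owner, through messages, to equip it or apply potion effects.
; Slot writes broadcast an inventory-changed event; pickup and HasItem are empty stubs.
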(event `self.ReceiveBeginPlay`
  (set `self.Owner` (`self.GetOwner`))
  (`self.Init Inventory`))

(event `Event_InventoryChanged`
  (params (Slot :type Integer))
  (`self.OnInventoryChanged` Slot))

(fn `Add Item to Slot`
  (params (`Item to Add` :type "/Game/RPG_Data/DA_ItemData Object Reference") (`Add to Slot` :type Integer) (Quantity :type Integer))
  (returns (Overflow :type Integer))
  (locals (Remaining :type Integer :default 0))
  (bind _max_stack (`/Game/RPG_Data/DA_ItemData.Max Stack` (`local.Item to Add`)))
  (bind (_return_value _return_remaining) (`/Game/RPG_StatSystem/StatsHelper.FL_Clamp (Integer)` (`local.Quantity`) 0 _max_stack))
  (set `local.Remaining` _return_remaining)
  (if (> _return_value 0)
    (bind _structout (setmembers `/Game/RPG_Data/Structs/S_ItemData` :`StructRef` (`BlueprintMapLibrary.Map_Find` (`self.Slot`) `Add to Slot`) :`Item` (`local.Item to Add`) :`Quantity` _return_value :`IsFull` (== _return_value _max_stack)))
    (`BlueprintMapLibrary.Map_Add` (`self.Slot`) (`local.Add to Slot`) _structout)
    (`self.Event_InventoryChanged` (`local.Add to Slot`))
    (return (`local.Remaining`))
    (else
      (`self.Clear Slot` (`local.Add to Slot`)))))

(fn `Add Slot Value`
  (params (Slot :type Integer) (Value :type "/Game/RPG_Data/Structs/S_ItemData Structure (by ref)"))
  (locals (`Source Item` :type "/Game/RPG_Data/Structs/S_ItemData Structure") (`Target Item` :type "/Game/RPG_Data/Structs/S_ItemData Structure"))
  (`BlueprintMapLibrary.Map_Add` (`self.Slot`) Slot Value)
  (`self.Event_InventoryChanged` (`local.Slot`)))

(fn `Check if Slot is Full`
  (params (Slot :type Integer))
  (returns (IsFull :type Boolean))
  (bind ((`Item_2_CDDDA1024B740CBE6EF48EBD56BC7EE3` _item) (`Quantity_7_8C0C0B6C4F3EF3EAB652F8A8D517110D` _quantity)) (break `/Game/RPG_Data/Structs/S_ItemData` (`BlueprintMapLibrary.Map_Find` (`self.Slot`) Slot)))
  (if (`KismetSystemLibrary.IsValid` _item)
    (if (>= _quantity (`/Game/RPG_Data/DA_ItemData.Max Stack` _item))
      (return true)
      (else
        (return false)))))

(fn `Clear Slot`
  (params (Slot :type Integer))
  (`BlueprintMapLibrary.Map_Add` (`self.Slot`) Slot (make `/Game/RPG_Data/Structs/S_ItemData` null))
  (`self.Event_InventoryChanged` (`local.Slot`))
  (return))

(fn `Debug Inventory`
  (params (`Print Debug` :type Boolean))
  (if `Print Debug`
    (bind _keys (`BlueprintMapLibrary.Map_Keys` (`self.Slot`)))
    (for _array_element _keys
      (bind ((`Item_2_CDDDA1024B740CBE6EF48EBD56BC7EE3` _item) (`Quantity_7_8C0C0B6C4F3EF3EAB652F8A8D517110D` _quantity)) (break `/Game/RPG_Data/Structs/S_ItemData` (`BlueprintMapLibrary.Map_Find` (`self.Slot`) _array_element)))
      (`KismetSystemLibrary.PrintString` (`KismetTextLibrary.Conv_TextToString` (`|FormatText` "Inventory \nSlot: {slot}, Item: {item}, Quantity {amount}" _array_element _item _quantity)) true true (struct :`G` 0.223108 :`B` 1.0 :`A` 1.0) 0.0))))

(fn `Drop Item to Ground`
  (params (`Item to Drop` :type "/Game/RPG_Data/DA_ItemData Object Reference") (Quantity :type Integer :default 1))
  (bind _returnvalue (`Actor.GetTransform` (`self.Owner`)))
  (bind _returnvalue_2 (`|SpawnActorFromClass` (`/Game/RPG_Data/DA_ItemData.Spawn Actor` `Item to Drop`) (`KismetMathLibrary.MakeTransform` (`KismetMathLibrary.MakeVector` (+ (.x (.location _returnvalue)) 75.0) (.y (.location _returnvalue)) (.z (.location _returnvalue))) (.rotation _returnvalue) (.scale _returnvalue)) "AlwaysSpawn" "MultiplyWithRoot" null (`local.Item to Drop`) false null))
  (`/Game/RPG_EquipmentSystem/BP_MasterEquipment.Set Collision` _returnvalue_2 false))

(fn `Fill Empty Slots`
  (params (`Item to Add` :type "/Game/RPG_Data/DA_ItemData Object Reference") (Quantity :type Integer :default 1))
  (locals (FoundEmptySlot :type Integer) (`Remaining Quantity` :type Integer :default 1))
  (set `local.Remaining Quantity` Quantity)
  (bind _keys (`BlueprintMapLibrary.Map_Keys` (`self.Slot`)))
  (for _array_element _keys
    (if (not (or (== (`local.Remaining Quantity`) 0) (not (`self.Is Slot Empty` _array_element))))
      (bind _overflow (`self.Add Item to Slot` (`local.Item to Add`) _array_element (`local.Remaining Quantity`)))
      (set `local.Remaining Quantity` _overflow)))
  (return))

(fn `Fill Existing Stacks`
  (params (`Item Data` :type "/Game/RPG_Data/DA_ItemData Object Reference") (Quantity :type Integer))
  (returns (Overflow :type Integer))
  (locals (`Incoming Quantity` :type Integer))
  (set `local.Incoming Quantity` Quantity)
  (bind _keys (`BlueprintMapLibrary.Map_Keys` (`self.Slot`)))
  (for _array_element _keys
    (if (== (`.Item_2_CDDDA1024B740CBE6EF48EBD56BC7EE3` (break `/Game/RPG_Data/Structs/S_ItemData` (`BlueprintMapLibrary.Map_Find` (`self.Slot`) _array_element))) (`local.Item Data`))
      (bind _remaining (`self.Modify Quantity` _array_element (`local.Incoming Quantity`)))
      (set `local.Incoming Quantity` _remaining)))
  (return (`local.Incoming Quantity`)))

(fn `Get First Empty Slot`
  (returns (ReturnValue :type Boolean) (`Empty Slot` :type Integer))
  (locals (Return :type Boolean :default false) (SlotNum :type Integer))
  (bind _keys (`BlueprintMapLibrary.Map_Keys` (`self.Slot`)))
  (for _array_element _keys
    (bind _returnvalue (`self.Is Slot Empty` _array_element))
    (if _returnvalue
      (set `local.Return` _returnvalue)
      (set `local.SlotNum` _array_element)
      (break)))
  (if (`local.Return`)
    (return true (`local.SlotNum`))
    (else
      (return false -1))))

(fn `Get First Matching Item`
  (params (`Item Data` :type "/Game/RPG_Data/DA_ItemData Object Reference") (`Look for Stackable` :type Boolean))
  (returns (`Item Found` :type Boolean) (Slot :type Integer))
  (locals (`Found Item in Slot` :type Integer :default -1) (Found :type Boolean))
  (bind _keys (`BlueprintMapLibrary.Map_Keys` (`self.Slot`)))
  (for _array_element _keys
    (bind ((`Item_2_CDDDA1024B740CBE6EF48EBD56BC7EE3` _item)) (break `/Game/RPG_Data/Structs/S_ItemData` (`BlueprintMapLibrary.Map_Find` (`self.Slot`) _array_element)))
    (if (== _item (`local.Item Data`))
      (if (`local.Look for Stackable`)
        (if (`/Game/RPG_Data/DA_ItemData.Is Item Stackable?` _item)
          (set `local.Found` true :!label _label)
          (set `local.Found Item in Slot` _array_element)
          (break))
        (else
          (goto _label)))))
  (if (`local.Found`)
    (return true (`local.Found Item in Slot`))
    (else
      (return false -1))))

(fn `Get Free Space at Slot`
  (params (Slot :type Integer))
  (returns (ReturnValue :type Integer))
  (return (- (`/Game/RPG_Data/DA_ItemData.Max Stack` (`self.Get Item At Slot` Slot)) (`self.Get Quantity At Slot` Slot))))

(fn `Get Item At Slot`
  (params (Slot :type Integer))
  (returns (Item :type "/Game/RPG_Data/DA_ItemData Object Reference"))
  (bind ((`Item_2_CDDDA1024B740CBE6EF48EBD56BC7EE3` _item)) (break `/Game/RPG_Data/Structs/S_ItemData` (`BlueprintMapLibrary.Map_Find` (`self.Slot`) Slot)))
  (if (`KismetSystemLibrary.IsValid` _item)
    (return _item)
    (else
      (return null))))

(fn `Get item struct`
  (params (Slot :type Integer))
  (returns (Item :type "/Game/RPG_Data/Structs/S_ItemData Structure"))
  (return (`BlueprintMapLibrary.Map_Find` (`self.Slot`) Slot)))

(fn `Get Quantity At Slot`
  (params (Slot :type Integer))
  (returns (Quantity :type Integer))
  (bind ((`Quantity_7_8C0C0B6C4F3EF3EAB652F8A8D517110D` _quantity)) (break `/Game/RPG_Data/Structs/S_ItemData` (`BlueprintMapLibrary.Map_Find` (`self.Slot`) Slot)))
  (if (> _quantity 0)
    (return _quantity)
    (else
      (return 0))))

(fn `Has Free Space`
  (params (Slot :type Integer))
  (returns (ReturnValue :type Boolean))
  (return (> (`/Game/RPG_Data/DA_ItemData.Max Stack` (`self.Get Item At Slot` Slot)) (`self.Get Quantity At Slot` Slot))))

(fn `Has Item`
  (params (`Item Data` :type "/Game/RPG_Data/DA_ItemData Object Reference")))

(fn `Init Inventory`
  (returns (Success :type Boolean))
  (for _index (range (`self.Inventory Size`))
    (`BlueprintMapLibrary.Map_Add` (`self.Slot`) _index (make `/Game/RPG_Data/Structs/S_ItemData` null)))
  (return (== (`BlueprintMapLibrary.Map_Length` (`self.Slot`)) (- (`self.Inventory Size`) 1))))

(fn `Is Slot Empty`
  (params (Slot :type "Integer (by ref)"))
  (returns (ReturnValue :type Boolean))
  (bind (_value _returnvalue) (`BlueprintMapLibrary.Map_Find` (`self.Slot`) Slot))
  (bind ((`Item_2_CDDDA1024B740CBE6EF48EBD56BC7EE3` _item) (`Quantity_7_8C0C0B6C4F3EF3EAB652F8A8D517110D` _quantity)) (break `/Game/RPG_Data/Structs/S_ItemData` _value))
  (if _returnvalue
    (if (or (not (`KismetSystemLibrary.IsValid` _item)) (<= _quantity 0))
      (return true)
      (else
        (return false)))))

(fn `Modify Quantity`
  (params (Slot :type Integer) (Amount :type Integer :default 1) (Decrease :type Boolean))
  (returns (Remaining :type Integer))
  (locals (RemainingAmount :type Integer :default 0))
  (bind _slot (`local.Slot`))
  (bind (_return_value _return_remaining) (`/Game/RPG_StatSystem/StatsHelper.FL_Clamp (Integer)` (+ (`self.Get Quantity At Slot` _slot) (`local.Amount`)) 0 (`/Game/RPG_Data/DA_ItemData.Max Stack` (`self.Get Item At Slot` _slot))))
  ; This function assumes item already exists in the slot
  (if Decrease
    (if (> (`self.Get Quantity At Slot` (`local.Slot`)) 0)
      (set `local.RemainingAmount` (- (`self.Get Quantity At Slot` (`local.Slot`)) (`local.Amount`)))
      (bind _structout (setmembers `/Game/RPG_Data/Structs/S_ItemData` :`StructRef` (`BlueprintMapLibrary.Map_Find` (`self.Slot`) (`local.Slot`)) :`Quantity` (`local.RemainingAmount`)))
      (`BlueprintMapLibrary.Map_Add` (`self.Slot`) (`local.Slot`) _structout)
      ; If Quantity reaches 0, we clear the slot
      (if (== (`self.Get Quantity At Slot` (`local.Slot`)) 0)
        (`self.Clear Slot` (`local.Slot`))
        (return 0)
        (else
          (`self.Event_InventoryChanged` (`local.Slot`))
          (return (`local.RemainingAmount`)))))
    (elif (not (`self.Check if Slot is Full` (`local.Slot`)))
      (set `local.RemainingAmount` _return_remaining)
      (bind _structout_2 (setmembers `/Game/RPG_Data/Structs/S_ItemData` :`StructRef` (`BlueprintMapLibrary.Map_Find` (`self.Slot`) (`local.Slot`)) :`Quantity` _return_value :`IsFull` (> _return_remaining 0)))
      (`BlueprintMapLibrary.Map_Add` (`self.Slot`) (`local.Slot`) _structout_2)
      (`self.Event_InventoryChanged` (`local.Slot`))
      (return (`local.RemainingAmount`))
      (else
        (return (`local.Amount`))))))

(fn `OnDrop`
  (params (`Source Slot` :type Integer) (`Target Slot` :type Integer))
  (locals (`Source Item Struct` :type "/Game/RPG_Data/Structs/S_ItemData Structure") (`Target Item Struct` :type "/Game/RPG_Data/Structs/S_ItemData Structure"))
  (bind _source_slot (`local.Source Slot`))
  (if (!= `Source Slot` `Target Slot`)
    (if (`self.Is Slot Empty` (`local.Target Slot`))
      (`BlueprintMapLibrary.Map_Add` (`self.Slot`) (`local.Target Slot`) (`self.Get item struct` (`local.Source Slot`)))
      (`self.Event_InventoryChanged` (`local.Target Slot`))
      (`self.Clear Slot` _source_slot)
      (`self.Event_InventoryChanged` _source_slot)
      (elif (== (`self.Get Item At Slot` (`local.Source Slot`)) (`self.Get Item At Slot` (`local.Target Slot`)))
        (if (`/Game/RPG_Data/DA_ItemData.Is Item Stackable?` (`self.Get Item At Slot` (`local.Target Slot`)))
          (`self.Stack Items` (`local.Source Slot`) (`local.Target Slot`)))
        (else
          ; If items at slots are not the same, we swap their places.
          (set `local.Source Item Struct` (`self.Get item struct` (`local.Source Slot`)))
          (set `local.Target Item Struct` (`self.Get item struct` (`local.Target Slot`)))
          (`self.Add Slot Value` (`local.Target Slot`) (`local.Source Item Struct`))
          (`self.Add Slot Value` (`local.Source Slot`) (`local.Target Item Struct`)))))))

(fn `Pick Up Item from Ground`)

(fn `Slot Has Free Space`
  (params (Slot :type Integer))
  (returns (ReturnValue :type Boolean))
  (bind _quantity (`self.Get Quantity At Slot` Slot))
  (return (== (`.Return Remaining` (`/Game/RPG_StatSystem/StatsHelper.FL_Clamp (Integer)` _quantity _quantity (`/Game/RPG_Data/DA_ItemData.Max Stack` (`self.Get Item At Slot` Slot)))) 0)))

(fn `Stack Items`
  (params (`Source Slot` :type Integer) (`Target Slot` :type Integer))
  (locals (`Target Data` :type "/Game/RPG_Data/Structs/S_ItemData Structure") (`Source Data` :type "/Game/RPG_Data/Structs/S_ItemData Structure"))
  (bind ((`Item_2_CDDDA1024B740CBE6EF48EBD56BC7EE3` _item) (`Quantity_7_8C0C0B6C4F3EF3EAB652F8A8D517110D` _quantity)) (break `/Game/RPG_Data/Structs/S_ItemData` (`local.Source Data`)))
  (`|ExecutionSequence`
    (:`then_0`
      (set `local.Target Data` (`self.Get item struct` (`local.Target Slot`)))
      (set `local.Source Data` (`self.Get item struct` (`local.Source Slot`))))
    (:`then_1`
      (bind _overflow (`self.Add Item to Slot` _item (`local.Target Slot`) (+ _quantity (`.Quantity_7_8C0C0B6C4F3EF3EAB652F8A8D517110D` (break `/Game/RPG_Data/Structs/S_ItemData` (`local.Target Data`))))))
      (`self.Add Item to Slot` (`.Item_2_CDDDA1024B740CBE6EF48EBD56BC7EE3` (break `/Game/RPG_Data/Structs/S_ItemData` (`local.Source Data`))) (`local.Source Slot`) _overflow))))

(fn `Try Add Item`
  (params (`Item to Add` :type "/Game/RPG_Data/DA_ItemData Object Reference") (Quantity :type Integer :default 1))
  (locals (`Has Free Slot` :type Boolean :default false) (StackableSlot :type Integer :default 0) (FoundEmptySlot :type Integer))
  (if (`self.Get First Matching Item` `Item to Add` true)
    (bind _overflow (`self.Fill Existing Stacks` (`local.Item to Add`) (`local.Quantity`)))
    (`self.Fill Empty Slots` (`local.Item to Add`) _overflow)
    (else
      (`self.Fill Empty Slots` (`local.Item to Add`) (`local.Quantity`)))))

(fn `Use Item from Slot`
  (params (Slot :type Integer))
  (returns (Success :type Boolean))
  (bind _item (`self.Get Item At Slot` (`local.Slot`)))
  (switch `/Game/RPG_Data/Enums/E_ItemCategory` (`/Game/RPG_Data/DA_ItemData.Item Category` (`self.Get Item At Slot` Slot))
    (:`NewEnumerator1`
      (bind _success (message `/Game/RPG_EquipmentSystem/BPI_Equipment.Equip Item` (`self.Owner`) (`self.Get Item At Slot` (`local.Slot`))))
      (if _success
        (`self.Clear Slot` (`local.Slot`))
        (return true)
        (else
          (return false))))
    (:`NewEnumerator2`
      (switch `/Game/RPG_Data/Enums/E_ConsumableType` (`/Game/RPG_Data/DA_ItemData.Consumable Type` (`self.Get Item At Slot` (`local.Slot`)))
        (:`NewEnumerator1`
          _)
        (:`NewEnumerator2`
          _)
        (:`NewEnumerator3`
          _))
      (bind _success_2 (message `/Game/RPG_StatSystem/BPI_Stats.Modify Derived Attributes` (`self.Owner`) (`/Game/RPG_Data/DA_ItemData.Derived Stat To Affect` _item) (`/Game/RPG_Data/DA_ItemData.Operation` _item) (`KismetMathLibrary.MakeVector2D` (`/Game/RPG_Data/DA_ItemData.Amount` _item))))
      (if _success_2
        (`self.Modify Quantity` (`local.Slot`) 1 true)))))