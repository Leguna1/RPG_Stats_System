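; Actor component that stores core stats as value/max pairs and broadcasts changes for UI updates.
; Looping timers regenerate health, stamina and mana, each started at BeginPlay only if below max.
; ChangeCoreStat applies instant, over-time or temporary modifications through ModifyAttribute, with timers counting down per-stat durations.
; Temporary changes restore a saved snapshot of the stat on expiry, while equipment attributes add or remove value and max bonuses.
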(event `self.ReceiveBeginPlay`
  ;[0.526 0.526 0.526 0.5] Begin Play
  (`self.Start Health Regeneration`)
  (`self.Start Stamina Regeneration`)
  (`self.Start Mana Regeneration`)
  (bind _keys (`BlueprintMapLibrary.Map_Keys` (`self.Core Stats`)))
  (for _array_element _keys
    (`self.UpdateCoreStatChange` _array_element)))

(event `Start Overtime Change`
  (params (Stat :type "/Game/Data/Enums/E_CoreStat Enum" :default "NewEnumerator0") (Type :type "/Game/Data/Enums/E_ValueType Enum" :default "NewEnumerator0") (Operation :type "/Game/Data/Enums/E_Operation Enum" :default "NewEnumerator0") (Interval :type "Float (double-precision)") (Duration :type "Float (double-precision)") (Amount :type "Float (double-precision)"))
  ;[0.4844 0.4844 0.4844 0.5] Overtime Change timer
  (`BlueprintMapLibrary.Map_Add` (`self.OvertimeDurations`) Stat Duration)
  (bind _returnvalue (`KismetSystemLibrary.K2_SetTimerDelegate` (`|CreateDelegate` :!event `TickOvertime Change`) Interval true))
  (set `self.OvertimeHandle` _returnvalue))

(event `TickOvertime Change`
  ;[0.4844 0.4844 0.4844 0.5] Overtime Change timer
  (bind _keys (`BlueprintMapLibrary.Map_Keys` (`self.OvertimeDurations`)))
  (for _array_element _keys
    (`self.Overtime` _array_element (stale `Start Overtime Change` Interval)
      (:`Removed`
        _)
      (:`Updated`
        (`self.Modify Attribute` (stale `Start Overtime Change` Stat) (stale `Start Overtime Change` Type) (stale `Start Overtime Change` Operation) (stale `Start Overtime Change` Amount))))
    (`self.UpdateCoreStatChange` (stale `Start Overtime Change` Stat)))
  (if (<= (`BlueprintMapLibrary.Map_Length` (`self.OvertimeDurations`)) 0)
    (`KismetSystemLibrary.K2_ClearAndInvalidateTimerHandle` (`self.OvertimeHandle`))))

(event `Start Temporary Change`
  (params (Stat :type "/Game/Data/Enums/E_CoreStat Enum" :default "NewEnumerator0") (Duration :type "Float (double-precision)"))
  ;[0.4375 0.4375 0.4375 0.5] Temporary incrase & decrease duration timer
  (`BlueprintMapLibrary.Map_Add` (`self.TemporaryDurations`) Stat Duration)
  (bind _returnvalue (`KismetSystemLibrary.K2_SetTimerDelegate` (`|CreateDelegate` :!event `TickDuration`) 1.0 true))
  (set `self.DurationTimerHandle` _returnvalue))

(event `TickDuration`
  ;[0.4375 0.4375 0.4375 0.5] Temporary incrase & decrease duration timer
  (bind _keys (`BlueprintMapLibrary.Map_Keys` (`self.TemporaryDurations`)))
  (for _array_element _keys
    (`self.Temporary` _array_element
      (:`Removed`
        _)
      (:`Updated`
        _))
    (`self.UpdateCoreStatChange` _array_element))
  (if (<= (`BlueprintMapLibrary.Map_Length` (`self.TemporaryDurations`)) 0)
    (`KismetSystemLibrary.K2_ClearAndInvalidateTimerHandle` (`self.DurationTimerHandle`))))

(event `UpdateCoreStatChange`
  (params (Stat :type "/Game/Data/Enums/E_CoreStat Enum" :default "NewEnumerator0"))
  ;[0.4844 0.4844 0.4844 0.5] Update UI
  (`self.OnCoreStatChanged` Stat (`self.Get Core Stat Values` Stat)))

(event `Start Health Regeneration`
  (bind (_values_value _values_maxvalue) (break `/Game/Data/Structs/S_StatValue` (`self.Get Core Stat Values` "NewEnumerator1")))
  (if (< _values_value _values_maxvalue)
    (bind _returnvalue (`KismetSystemLibrary.K2_SetTimerDelegate` (`|CreateDelegate` :!event `Health Regeneration`) (`self.Health Regen Speed`) true))
    (set `self.Health Regen Timer` _returnvalue)))

(event `Start Stamina Regeneration`
  (bind (_values_value _values_maxvalue) (break `/Game/Data/Structs/S_StatValue` (`self.Get Core Stat Values` "NewEnumerator3")))
  (if (< _values_value _values_maxvalue)
    (bind _returnvalue (`KismetSystemLibrary.K2_SetTimerDelegate` (`|CreateDelegate` :!event `Stamina Regeneration`) (`self.Stamina Regen Speed`) true))
    (set `self.Stamina Regen Timer` _returnvalue)))

(event `Start Mana Regeneration`
  (bind (_values_value _values_maxvalue) (break `/Game/Data/Structs/S_StatValue` (`self.Get Core Stat Values` "NewEnumerator2")))
  (if (< _values_value _values_maxvalue)
    (bind _returnvalue (`KismetSystemLibrary.K2_SetTimerDelegate` (`|CreateDelegate` :!event `Mana Regeneration`) (`self.Mana Regen Speed`) true))
    (set `self.Mana Regen Timer` _returnvalue)))

(fn `Add Equipment Attributes`
  (params (`Equipped Attributes` :type "Map of /Game/Data/Enums/E_CoreStat Enum to /Game/Data/Structs/S_StatValue Structure") (Add :type Boolean))
  (locals (`Inc Stat Value` :type "Float (double-precision)") (`Equipment Attributes` :type "Map of /Game/Data/Enums/E_CoreStat Enum to /Game/Data/Structs/S_StatValue Structure") (`Inc Max Value` :type "Float (double-precision)"))
  (bind _add (`local.Add`))
  (set `local.Equipment Attributes` `Equipped Attributes`)
  (bind _keys (`BlueprintMapLibrary.Map_Keys` (`local.Equipment Attributes`)))
  (for _array_element _keys
    (bind (_value _returnvalue) (`BlueprintMapLibrary.Map_Find` (`local.Equipment Attributes`) _array_element))
    (if _returnvalue
      (bind (_value_2 _maxvalue) (break `/Game/Data/Structs/S_StatValue` _value))
      (set `local.Inc Stat Value` _value_2)
      (set `local.Inc Max Value` _maxvalue)
      (`self.Modify Attribute` _array_element "NewEnumerator1" (select `bool` _add :`false` "NewEnumerator2" :`true` "NewEnumerator1" :!type "/Game/Data/Enums/E_Operation Enum") (`local.Inc Stat Value`))
      (`self.Modify Attribute` _array_element "NewEnumerator3" (select `bool` _add :`false` "NewEnumerator2" :`true` "NewEnumerator1" :!type "/Game/Data/Enums/E_Operation Enum") (`local.Inc Max Value`))
      (`self.OnCoreStatChanged` _array_element (`self.Get Core Stat Values` _array_element))
      (else
        (return))))
  (return))

(fn `Change Core Stat`
  (params (Stat :type "/Game/Data/Enums/E_CoreStat Enum" :default "NewEnumerator0") (`Value Type` :type "/Game/Data/Enums/E_ValueType Enum" :default "NewEnumerator0") (`Change Options` :type "/Game/Data/Structs/S_StatEditor Structure"))
  (returns (Success :type Boolean))
  (locals (Amount :type "Float (double-precision)") (ReturnBase :type "Float (double-precision)" :default 0.0) (ReturnBonus :type "Float (double-precision)" :default 0.0) (DurationL :type "Float (double-precision)") (SpeedL :type "Float (double-precision)") (Operation :type "/Game/Data/Enums/E_Operation Enum"))
  (bind (_method _operation _amount _duration _speed) (break `/Game/Data/Structs/S_StatEditor` `Change Options`))
  (set `local.Operation` _operation)
  (set `local.Amount` _amount)
  (switch `/Game/Data/Enums/E_Method` _method
    (:`NewEnumerator0`
      (return false))
    (:`NewEnumerator1`
      (`self.Modify Attribute` (`local.Stat`) (`local.Value Type`) (`local.Operation`) (`local.Amount`))
      (`self.UpdateCoreStatChange` (`local.Stat`))
      (return true))
    (:`NewEnumerator4`
      (`self.Start Overtime Change` (`local.Stat`) (`local.Value Type`) (`local.Operation`) _speed _duration _amount)
      (`self.UpdateCoreStatChange` (`local.Stat`))
      (return true))
    (:`NewEnumerator3`
      (`self.SaveStat` (`local.Stat`))
      (`self.Modify Attribute` (`local.Stat`) (`local.Value Type`) (`local.Operation`) (`local.Amount`))
      (`self.Start Temporary Change` (`local.Stat`) _duration)
      (`self.UpdateCoreStatChange` (`local.Stat`))
      (return true))))

(fn `Get Core Stat Values`
  (params (Stat :type "/Game/Data/Enums/E_CoreStat Enum" :default "NewEnumerator0"))
  (returns (Values :type "/Game/Data/Structs/S_StatValue Structure"))
  (bind (_value _returnvalue) (`BlueprintMapLibrary.Map_Find` (`self.Core Stats`) Stat))
  (if _returnvalue
    (return _value)))

(fn `GetSavedStat`
  (params (Stat :type "/Game/Data/Enums/E_CoreStat Enum" :default "NewEnumerator0"))
  (returns (Value :type "/Game/Data/Structs/S_StatValue Structure"))
  (bind (_value _returnvalue) (`BlueprintMapLibrary.Map_Find` (`self.Save Stats`) Stat))
  (if _returnvalue
    (return _value)))

(fn `Health Regeneration`
  (locals (CurrentHealth :type "Float (double-precision)" :default 0.0) (MaxHealth :type "Float (double-precision)" :default 0.0))
  (bind (_values_value _values_maxvalue) (break `/Game/Data/Structs/S_StatValue` (`self.Get Core Stat Values` "NewEnumerator1")))
  (set `local.CurrentHealth` _values_value)
  (set `local.MaxHealth` _values_maxvalue)
  (set `local.CurrentHealth` (`KismetMathLibrary.FClamp` (+ (`local.CurrentHealth`) (`self.Health Regen Amount`)) 0.0 (`local.MaxHealth`)))
  (`BlueprintMapLibrary.Map_Add` (`self.Core Stats`) "NewEnumerator1" (make `/Game/Data/Structs/S_StatValue` (`local.CurrentHealth`) (`local.MaxHealth`)))
  (`self.UpdateCoreStatChange` "NewEnumerator1")
  (if (or (== (`local.CurrentHealth`) 0.0) (not (`self.IsAlive`)))
    (`KismetSystemLibrary.K2_ClearAndInvalidateTimerHandle` (`self.Health Regen Timer`))))

(fn `Mana Regeneration`
  (locals (CurrentMana :type "Float (double-precision)") (MaxMana :type "Float (double-precision)"))
  (bind (_values_value _values_maxvalue) (break `/Game/Data/Structs/S_StatValue` (`self.Get Core Stat Values` "NewEnumerator2")))
  (set `local.CurrentMana` _values_value)
  (set `local.MaxMana` _values_maxvalue)
  (set `local.CurrentMana` (`KismetMathLibrary.FClamp` (+ (`local.CurrentMana`) (`self.Mana Regen Amount`)) 0.0 (`local.MaxMana`)))
  (`BlueprintMapLibrary.Map_Add` (`self.Core Stats`) "NewEnumerator2" (make `/Game/Data/Structs/S_StatValue` (`local.CurrentMana`) (`local.MaxMana`)))
  (`self.UpdateCoreStatChange` "NewEnumerator2")
  (if (or (== (`local.CurrentMana`) 0.0) (not (`self.IsAlive`)))
    (`KismetSystemLibrary.K2_ClearAndInvalidateTimerHandle` (`self.Mana Regen Timer`))))

(fn `Modify Attribute`
  (params (Attribute :type "/Game/Data/Enums/E_CoreStat Enum" :default "NewEnumerator0") (`Value Type` :type "/Game/Data/Enums/E_ValueType Enum" :default "NewEnumerator0") (Operation :type "/Game/Data/Enums/E_Operation Enum" :default "NewEnumerator0") (`Modify Value` :type "Float (double-precision)"))
  (bind (_value _maxvalue) (break `/Game/Data/Structs/S_StatValue` (`BlueprintMapLibrary.Map_Find` (`self.Core Stats`) (`local.Attribute`))))
  (bind (_value_2 _maxvalue_2) (break `/Game/Data/Structs/S_StatValue` (`BlueprintMapLibrary.Map_Find` (`self.Core Stats`) (`local.Attribute`))))
  (switch `/Game/Data/Enums/E_ValueType` `Value Type`
    (:`NewEnumerator1`
      (bind _return_value (`/Game/MyFunctionLibrary.Call_Operator` (`local.Operation`) _value_2 (`local.Modify Value`)))
      (`BlueprintMapLibrary.Map_Add` (`self.Core Stats`) (`local.Attribute`) (make `/Game/Data/Structs/S_StatValue` _return_value _maxvalue_2))
      (return))
    (:`NewEnumerator3`
      (bind _return_value_2 (`/Game/MyFunctionLibrary.Call_Operator` (`local.Operation`) _maxvalue (`local.Modify Value`)))
      (`BlueprintMapLibrary.Map_Add` (`self.Core Stats`) (`local.Attribute`) (make `/Game/Data/Structs/S_StatValue` _value _return_value_2))
      (return))))

(fn `Set Stat Value`
  (params (Stat :type "/Game/Data/Enums/E_CoreStat Enum" :default "NewEnumerator0") (`Value Type` :type "/Game/Data/Enums/E_ValueType Enum" :default "NewEnumerator0") (`New Value` :type "Float (double-precision)"))
  (bind (_value _maxvalue) (break `/Game/Data/Structs/S_StatValue` (`BlueprintMapLibrary.Map_Find` (`self.Core Stats`) Stat)))
  (switch `/Game/Data/Enums/E_ValueType` `Value Type`
    (:`NewEnumerator1`
      (`BlueprintMapLibrary.Map_Add` (`self.Core Stats`) Stat (make `/Game/Data/Structs/S_StatValue` `New Value` _maxvalue)))
    (:`NewEnumerator3`
      (`BlueprintMapLibrary.Map_Add` (`self.Core Stats`) Stat (make `/Game/Data/Structs/S_StatValue` _value `New Value`)))))

(fn `Stamina Regeneration`
  (locals (CurrentStamina :type "Float (double-precision)") (MaxStamina :type "Float (double-precision)"))
  (bind (_values_value _values_maxvalue) (break `/Game/Data/Structs/S_StatValue` (`self.Get Core Stat Values` "NewEnumerator3")))
  (set `local.CurrentStamina` _values_value)
  (set `local.MaxStamina` _values_maxvalue)
  (set `local.CurrentStamina` (`KismetMathLibrary.FClamp` (+ (`local.CurrentStamina`) (`self.Stamina Regen Amount`)) 0.0 (`local.MaxStamina`)))
  (`BlueprintMapLibrary.Map_Add` (`self.Core Stats`) "NewEnumerator3" (make `/Game/Data/Structs/S_StatValue` (`local.CurrentStamina`) (`local.MaxStamina`)))
  (`self.UpdateCoreStatChange` "NewEnumerator3")
  (if (or (== (`local.CurrentStamina`) 0.0) (not (`self.IsAlive`)))
    (`KismetSystemLibrary.K2_ClearAndInvalidateTimerHandle` (`self.Stamina Regen Timer`))))