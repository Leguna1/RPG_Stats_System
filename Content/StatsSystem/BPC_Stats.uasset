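; Stats component that manages a character's health, damage intake, death state and regeneration, following an observer pattern.
; TakeMigratedDamage rolls attack or magic power, mitigates it by armor or magic resist scaled with level, then applies an elemental matchup multiplier.
; It calls damage response, then death or RegenerateHealth, which heals random amounts on a looping timer and calls UI updates.
; TakeDoT only subtracts damage divided by duration once, without clamping or death checks.
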(event `self.ReceiveBeginPlay`
  ;[1 1 1] This component follows single responsiblity and observer pattern design principles.
)

(fn `CanBeDamaged?`
  (returns (Return :type Boolean))
  (if (not (and (`self.IsDead`) (`self.DamageImmune`)))
    (return true)))

(fn `GetElementMultiplier`
  (params (`Offensive Element` :type "/Game/StatsSystem/Variables/E_Element Enum" :default "NewEnumerator2") (`Defensive Element` :type "/Game/StatsSystem/Variables/E_Element Enum" :default "NewEnumerator2"))
  (returns (Multiplier :type "Float (double-precision)"))
  (switch `/Game/StatsSystem/Variables/E_Element` `Offensive Element`
    (:`NewEnumerator2`
      (switch `/Game/StatsSystem/Variables/E_Element` `Defensive Element`
        (:`NewEnumerator2`
          (set `self.ElementPower` 1.0))
        (:`NewEnumerator3`
          (set `self.ElementPower` 0.5 :!label _label))
        (:`NewEnumerator4`
          (goto _label))
        (:`NewEnumerator5`
          (goto _label))
        (:`NewEnumerator6`
          (goto _label)))
      (return (`self.ElementPower`)))
    (:`NewEnumerator3`
      (switch `/Game/StatsSystem/Variables/E_Element` `Defensive Element`
        (:`NewEnumerator2`
          (set `self.ElementPower` 1.3))
        (:`NewEnumerator3`
          (set `self.ElementPower` 1.0 :!label _label_2))
        (:`NewEnumerator4`
          (set `self.ElementPower` 0.3))
        (:`NewEnumerator5`
          (goto _label_2))
        (:`NewEnumerator6`
          (set `self.ElementPower` 1.5)))
      (return (`self.ElementPower`)))
    (:`NewEnumerator4`
      (switch `/Game/StatsSystem/Variables/E_Element` `Defensive Element`
        (:`NewEnumerator2`
          (set `self.ElementPower` 0.5))
        (:`NewEnumerator3`
          (set `self.ElementPower` 1.5))
        (:`NewEnumerator4`
          (set `self.ElementPower` 1.0 :!label _label_3))
        (:`NewEnumerator5`
          (set `self.ElementPower` 0.3))
        (:`NewEnumerator6`
          (goto _label_3)))
      (return (`self.ElementPower`)))
    (:`NewEnumerator5`
      (switch `/Game/StatsSystem/Variables/E_Element` `Defensive Element`
        (:`NewEnumerator2`
          (set `self.ElementPower` 0.5))
        (:`NewEnumerator3`
          (set `self.ElementPower` 1.0 :!label _label_4))
        (:`NewEnumerator4`
          (set `self.ElementPower` 1.5))
        (:`NewEnumerator5`
          (goto _label_4))
        (:`NewEnumerator6`
          (set `self.ElementPower` 0.3)))
      (return (`self.ElementPower`)))
    (:`NewEnumerator6`
      (switch `/Game/StatsSystem/Variables/E_Element` `Defensive Element`
        (:`NewEnumerator2`
          (set `self.ElementPower` 1.3))
        (:`NewEnumerator3`
          (set `self.ElementPower` 0.3))
        (:`NewEnumerator4`
          (set `self.ElementPower` 1.0 :!label _label_5))
        (:`NewEnumerator5`
          (set `self.ElementPower` 1.5))
        (:`NewEnumerator6`
          (goto _label_5)))
      (return (`self.ElementPower`)))))

(fn `InvertValue`
  (params (Value :type "Float (double-precision)") (`True?` :type Boolean))
  (returns (`Return Value` :type "Float (double-precision)"))
  (if `True?`
    (return Value)
    (else
      (return (* Value -1.0)))))

(fn `MitigateDamage`
  (params (DamageType :type "/Game/StatsSystem/Variables/E_DamageType Enum" :default "NewEnumerator5") (`Attack Power` :type "Float (double-precision)") (`Magic Power` :type "Float (double-precision)") (`Armor Value` :type "Float (double-precision)") (`Magic Resist Value` :type "Float (double-precision)") (`Character Level` :type Integer))
  (returns (`Return Value` :type "Float (double-precision)"))
  (switch `/Game/StatsSystem/Variables/E_DamageType` DamageType
    (:`NewEnumerator5`
      _)
    (:`NewEnumerator6`
      _)
    (:`NewEnumerator7`
      (return (* (`local.Magic Power`) (- 1.0 (/ (`local.Magic Resist Value`) (+ (`local.Magic Resist Value`) (* (`local.Character Level`) (`self.Balance FactorK`)))))))))
  (return (* (`local.Attack Power`) (- 1.0 (/ (`local.Armor Value`) (+ (`local.Armor Value`) (* (`local.Character Level`) (`self.Balance FactorK`))))))))

(fn `RegenerateHealth`
  (bind _maxhealth (`self.MaxHealth`))
  (bind _returnvalue (`KismetMathLibrary.RandomFloatInRange` (/ (`self.Health Regen Amount`) 2.0) (`self.Health Regen Amount`)))
  (if (< (`self.Health`) (`self.MaxHealth`))
    (bind _returnvalue_2 (`KismetSystemLibrary.K2_SetTimer` null "RegenerateHealth" (`KismetMathLibrary.RandomFloatInRange` (/ (`self.HealthRegenTime`) 2.0) (`self.HealthRegenTime`)) true))
    (set `self.RegenTimerHandle` _returnvalue_2)
    (bind _output_get (set `self.Health` (`KismetMathLibrary.FClamp` (+ (`self.Health`) _returnvalue) 0.0 _maxhealth)))
    (`self.OnUpdateUI` _output_get _maxhealth _returnvalue)
    (else
      (`KismetSystemLibrary.K2_ClearAndInvalidateTimerHandle` (`self.RegenTimerHandle`))
      (`KismetSystemLibrary.PrintString` "Timer Cleared"))))

(fn `TakeDoT`
  (params (DamageDealer :type "Actor Object Reference") (DamageAmount :type "Float (double-precision)") (Duration :type "Float (double-precision)"))
  (if (`self.CanBeDamaged?`)
    (set `self.Health` (- (`self.Health`) (/ DamageAmount Duration)))))

(fn `TakeMigratedDamage`
  (params (`Damage Dealer` :type "Actor Object Reference") (`Damage Type` :type "/Game/StatsSystem/Variables/E_DamageType Enum" :default "NewEnumerator5") (`Damage Info` :type "/Game/StatsSystem/Variables/S_OffensivePower Structure"))
  (bind (_weaponelement _attackpowermin _attackpowermax _magicpowermin _magicpowermax) (break `/Game/StatsSystem/Variables/S_OffensivePower` `Damage Info`))
  (bind (_defensiveelement _armor _magicresist) (break `/Game/StatsSystem/Variables/S_DefensivePower` (`self.Defensive Power`)))
  (bind _returnvalue (* (`self.GetElementMultiplier` _weaponelement _defensiveelement) (`self.MitigateDamage` `Damage Type` (`KismetMathLibrary.RandomFloatInRange` _attackpowermin _attackpowermax) (`KismetMathLibrary.RandomFloatInRange` _magicpowermin _magicpowermax) _armor _magicresist (`self.Character Level`))))
  (if (`self.CanBeDamaged?`)
    (set `self.Health` (`KismetMathLibrary.FClamp` (- (`self.Health`) _returnvalue) 0.0 (`self.MaxHealth`)))
    (`self.OnDamageResponse` (`local.Damage Dealer`) _returnvalue (`local.Damage Type`))
    (bind _output_get (set `self.IsDead` (>= _returnvalue (`self.Health`))))
    (if _output_get
      (`self.OnDeath` (`local.Damage Dealer`))
      (else
        (`self.RegenerateHealth`)))))