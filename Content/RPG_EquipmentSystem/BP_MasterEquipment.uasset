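; BP_MasterEquipment is a base equipment actor in the RPG equipment system, configured from its Data variable.
; On BeginPlay it applies the mesh, then, if that succeeds, copies core and derived attribute sets and attaches any activation VFX at "Socket One".
; SetCollision records equipped state, disabling collision and physics when equipped.
; When unequipped, it enables both, then stops physics simulation after a short delay.
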(event `self.ReceiveBeginPlay`
  (bind _data (`self.Data`))
  (bind _activation_vfx (`/Game/RPG_Data/DA_ItemData.Activation VFX` (`self.Data`)))
  (bind _returnvalue (`StaticMeshComponent.SetStaticMesh` (`self.StaticMesh`) (`/Game/RPG_Data/DA_ItemData.Static Mesh` (`self.Data`))))
  (if _returnvalue
    (set `self.Core Attribute Set` (`/Game/RPG_Data/DA_ItemData.Equipment Core Attributes` _data))
    (set `self.Derived Attribute Set` (`/Game/RPG_Data/DA_ItemData.Equipment Derived Attributes` _data))
    (if (`KismetSystemLibrary.IsValid` _activation_vfx)
      (`NiagaraFunctionLibrary.SpawnSystemAttached` _activation_vfx (`self.StaticMesh`) "Socket One" (`SceneComponent.GetSocketLocation` (`self.StaticMesh`) "Socket One") (struct) "SnapToTarget"))))

(event `Set Collision`
  (params (IsEquipped :type Boolean))
  (bind _staticmesh (`self.StaticMesh`))
  (bind _staticmesh_2 (`self.StaticMesh`))
  (bind _output_get (set `self.IsEquipped` IsEquipped))
  (if _output_get
    (`PrimitiveComponent.SetCollisionEnabled` _staticmesh "NoCollision")
    (`PrimitiveComponent.SetSimulatePhysics` _staticmesh false)
    (else
      (`PrimitiveComponent.SetCollisionEnabled` _staticmesh_2 "QueryAndPhysics")
      (`PrimitiveComponent.SetSimulatePhysics` _staticmesh_2 true)
      (`KismetSystemLibrary.Delay` 2.0)
      (`PrimitiveComponent.SetSimulatePhysics` _staticmesh_2 false))))

(fn `UserConstructionScript`)