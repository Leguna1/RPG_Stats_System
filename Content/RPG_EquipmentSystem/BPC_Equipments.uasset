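; Character equipment component that equips and unequips items in slots keyed by equipment type.
; Equipping checks class and level, clears an occupied slot, then spawns the item actor and attaches it to a mesh socket.
; Unequipping requires a successful inventory add before destroying the actor.
; Equip and unequip dispatchers drive stat changes, sending the item's core and derived attributes to the owner through interface messages.
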(event `self.ReceiveBeginPlay`
  (bind _output_get (set `self.Cached Owner` (`self.GetOwner`)))
  (bind _ascharacter (cast `Character` _output_get))
  (set `self.Owner Mesh` (`Character.Mesh` _ascharacter))
  (add `self.OnItemEquipped` (`|CreateDelegate` :!event `Event_ItemEquipped`))
  (add `self.OnItemUnequipped` (`|CreateDelegate` :!event `Event_Item Unequipped`)))

(event `Event_ItemEquipped` :!signature `self.OnItemEquipped`
  (params (Type :type "/Game/RPG_Data/Enums/E_ItemType Enum" :default "NewEnumerator0"))
  ; Update Character Stats with Equipment Stats
  (`self.Modify Stats` Type "NewEnumerator1"))

(event `Event_Item Unequipped` :!signature `self.OnItemUnequipped`
  (params (`Item Type` :type "/Game/RPG_Data/Enums/E_ItemType Enum" :default "NewEnumerator0"))
  ; Update Character Stats with Equipment Stats
  (`self.Modify Stats` `Item Type` "NewEnumerator8"))

(fn `Can Equip `
  (params (Data :type "/Game/RPG_Data/DA_ItemData Object Reference"))
  (returns (ReturnValue :type Boolean))
  (locals (`Current Level` :type Integer :default 0))
  (bind _level (message `/Game/RPG_StatSystem/BPI_Stats.Get_Current Level` (`self.Cached Owner`)))
  (set `local.Current Level` _level)
  (bind _class (message `/Game/RPG_StatSystem/BPI_Stats.Get Character Class` (`self.Cached Owner`)))
  (return (`/Game/RPG_Data/DA_ItemData.CanEquip?` (`local.Data`) _class (`local.Current Level`))))

(fn `Debug Equipments`
  (params (`Print Debug` :type Boolean))
  (bind _equipments (`self.Equipments`))
  (if `Print Debug`
    (bind _keys (`BlueprintMapLibrary.Map_Keys` _equipments))
    (for _array_element _keys
      (bind (_data _isequipped _equipmentinstane) (break `/Game/RPG_Data/Structs/S_Equipment` (`BlueprintMapLibrary.Map_Find` _equipments _array_element)))
      (`KismetSystemLibrary.PrintString` (`KismetTextLibrary.Conv_TextToString` (`|FormatText` "Equipment Type: {Type}, Data {Data}, Is Equipped {bool}, Instance: {Instance}" (`|GetEnumeratorNameAsString` _array_element) _data _isequipped _equipmentinstane)) true true (struct :`G` 0.66 :`B` 1.0 :`A` 1.0) 0.0))))

(fn `Get Equipped Item Instance`
  (params (`Item ID` :type "/Game/RPG_Data/Enums/E_ItemType Enum" :default "NewEnumerator0"))
  (returns (`Equipment Instane` :type "/Game/RPG_EquipmentSystem/BP_MasterEquipment Object Reference"))
  (bind (_value _returnvalue) (`BlueprintMapLibrary.Map_Find` (`self.Equipments`) `Item ID`))
  (if _returnvalue
    (return (`.EquipmentInstane_10_68E587A145C56B9F9FEFC89446A15790` (break `/Game/RPG_Data/Structs/S_Equipment` _value)))))

(fn `Get UI Data`
  (params (`Item ID` :type "/Game/RPG_Data/Enums/E_ItemType Enum" :default "NewEnumerator0"))
  (returns (`Display Name` :type Text) (Description :type Text) (`Icon Image` :type "Texture2D Object Reference"))
  (bind ((`Data_2_62C1816047F12CADE29F038DA5AE895C` _data) (`EquipmentInstane_10_68E587A145C56B9F9FEFC89446A15790` _equipmentinstane)) (break `/Game/RPG_Data/Structs/S_Equipment` (`BlueprintMapLibrary.Map_Find` (`self.Equipments`) `Item ID`)))
  (if (`KismetSystemLibrary.IsValid` _equipmentinstane)
    (return (`/Game/RPG_Data/DA_ItemData.Display Name` _data) (`/Game/RPG_Data/DA_ItemData.Description` _data) (`/Game/RPG_Data/DA_ItemData.Icon Image` _data))))

(fn `Modify Stats`
  (params (`Item ID` :type "/Game/RPG_Data/Enums/E_ItemType Enum" :default "NewEnumerator0") (Operation :type "/Game/RPG_Data/Enums/E_Operation Enum" :default "NewEnumerator0"))
  (locals (CoreAttributes :type "Map of /Game/RPG_Data/Enums/E_CoreStat Enum to /Game/RPG_Data/Structs/S_BaseBonus Structure") (DerivedAttributes :type "Map of /Game/RPG_Data/Enums/E_DerivedStat Enum to /Game/RPG_Data/Structs/S_BaseBonus Structure"))
  (bind _equipment_instane (`self.Get Equipped Item Instance` `Item ID`))
  (set `local.CoreAttributes` (`/Game/RPG_EquipmentSystem/BP_MasterEquipment.Core Attribute Set` _equipment_instane))
  (set `local.DerivedAttributes` (`/Game/RPG_EquipmentSystem/BP_MasterEquipment.Derived Attribute Set` _equipment_instane))
  (bind _keys (`BlueprintMapLibrary.Map_Keys` (`local.DerivedAttributes`)))
  (for _array_element _keys
    (bind (_basevalue _bonusvalue) (break `/Game/RPG_Data/Structs/S_BaseBonus` (`BlueprintMapLibrary.Map_Find` (`local.DerivedAttributes`) _array_element)))
    (message `/Game/RPG_StatSystem/BPI_Stats.Modify Derived Attributes` (`self.Cached Owner`) _array_element (`local.Operation`) (`KismetMathLibrary.MakeVector2D` _basevalue _bonusvalue)))
  (bind _keys_2 (`BlueprintMapLibrary.Map_Keys` (`local.CoreAttributes`)))
  (for _array_element_2 _keys_2
    (bind (_basevalue_2 _bonusvalue_2) (break `/Game/RPG_Data/Structs/S_BaseBonus` (`BlueprintMapLibrary.Map_Find` (`local.CoreAttributes`) _array_element_2)))
    (message `/Game/RPG_StatSystem/BPI_Stats.Modify Core Attributes` (`self.Cached Owner`) _array_element_2 (`local.Operation`) (`KismetMathLibrary.MakeVector2D` _basevalue_2 _bonusvalue_2)))
  (return))

(fn `Slot Is Empty`
  (params (`Item Data` :type "/Game/RPG_Data/DA_ItemData Object Reference"))
  (returns (ReturnValue :type Boolean))
  (bind _equipment_type (`/Game/RPG_Data/DA_ItemData.Equipment Type` `Item Data`))
  (bind (_value _returnvalue) (`BlueprintMapLibrary.Map_Find` (`self.Equipments`) _equipment_type))
  (if (and (`BlueprintMapLibrary.Map_Contains` (`self.Equipments`) _equipment_type) _returnvalue)
    (return (not (`.IsEquipped_6_5FD7D2214AEF35804085D1A97B4ED1F4` (break `/Game/RPG_Data/Structs/S_Equipment` _value))))))

(fn `Spawn Item`
  (params (`Item Data` :type "/Game/RPG_Data/DA_ItemData Object Reference"))
  (returns (`Spawned Item` :type "/Game/RPG_EquipmentSystem/BP_MasterEquipment Object Reference"))
  (bind _spawn_actor (`/Game/RPG_Data/DA_ItemData.Spawn Actor` `Item Data`)
    (:`then`
      (bind _returnvalue (`|SpawnActorFromClass` _spawn_actor (`KismetMathLibrary.MakeTransform` (0.0 0.0 0.0)) "AdjustIfPossibleButAlwaysSpawn" "MultiplyWithRoot" null `Item Data` false null))
      (return _returnvalue))
    (:`else`)))

(fn `Try Equip`
  (params (Data :type "/Game/RPG_Data/DA_ItemData Object Reference"))
  (returns (Success :type Boolean))
  (locals (`Item Instance` :type "/Game/RPG_EquipmentSystem/BP_MasterEquipment Object Reference"))
  (bind _data (`/Game/RPG_EquipmentSystem/BP_MasterEquipment.Data` (`local.Item Instance`)))
  (bind _equipment_type (`/Game/RPG_Data/DA_ItemData.Equipment Type` _data))
  (if (`self.Can Equip ` Data)
    (if (`self.Slot Is Empty` (`local.Data`))
      (bind _spawned_item (`self.Spawn Item` (`local.Data`) :!label _label))
      (bind _output_get (set `local.Item Instance` _spawned_item))
      (`/Game/RPG_EquipmentSystem/BP_MasterEquipment.Set Collision` _output_get true)
      (`Actor.K2_AttachToComponent` (`local.Item Instance`) (`self.Owner Mesh`) (`/Game/RPG_Data/DA_ItemData.Socket to Attach` (`/Game/RPG_EquipmentSystem/BP_MasterEquipment.Data` (`local.Item Instance`))) "SnapToTarget" "SnapToTarget" "SnapToTarget" true)
      (`BlueprintMapLibrary.Map_Add` (`self.Equipments`) _equipment_type (make `/Game/RPG_Data/Structs/S_Equipment` _data true (`local.Item Instance`)))
      (`self.OnItemEquipped` _equipment_type)
      (return true)
      (else
        (bind _success (`self.Try Unequip` (`local.Data`)))
        (if _success
          (goto _label))))
    (else
      (return false))))

(fn `Try Unequip`
  (params (`Item Data` :type "/Game/RPG_Data/DA_ItemData Object Reference"))
  (returns (Success :type Boolean))
  (locals (`Current Instance` :type "/Game/RPG_EquipmentSystem/BP_MasterEquipment Object Reference"))
  (bind ((`IsEquipped_6_5FD7D2214AEF35804085D1A97B4ED1F4` _isequipped) (`EquipmentInstane_10_68E587A145C56B9F9FEFC89446A15790` _equipmentinstane)) (break `/Game/RPG_Data/Structs/S_Equipment` (`BlueprintMapLibrary.Map_Find` (`self.Equipments`) (`/Game/RPG_Data/DA_ItemData.Equipment Type` `Item Data`))))
  (set `local.Current Instance` _equipmentinstane)
  (if _isequipped
    (bind _success (message `/Game/RPG_InventorySystem/BPI_Inventory.Add Item to Inventory` (`self.Cached Owner`) (`local.Item Data`) 1))
    (if _success
      (`self.OnItemUnequipped` (`/Game/RPG_Data/DA_ItemData.Equipment Type` (`local.Item Data`)))
      (`BlueprintMapLibrary.Map_Add` (`self.Equipments`) (`/Game/RPG_Data/DA_ItemData.Equipment Type` (`local.Item Data`)) (make `/Game/RPG_Data/Structs/S_Equipment` null false null))
      (`Actor.K2_DestroyActor` (`local.Current Instance`))
      (return true)
      (else
        (`KismetSystemLibrary.PrintString` "Inventory is full, cannot unequip item")
        (return false)))
    (else
      (return true))))