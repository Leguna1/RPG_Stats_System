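; Ability cooldown component that builds an ability map from SpellBook on BeginPlay and tracks which abilities are cooling down.
; TriggerCooldown adds an ability not already cooling down to the ActiveCooldown map and starts a looping timer.
; TickCooldown broadcasts OnUpdateCD, decrements each entry, removes expired ones and clears the timer once the map is empty.
; Attack, Eviscerate and StunCrash are example abilities gated by TriggerCooldown that only print text.
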(event `self.ReceiveBeginPlay`
  ;[0 0 0] Begin Play
  (for _array_element (`self.SpellBook`)
    (bind (_name _description _icon _cooldown) (break `/Game/ExampleTimer/S_AbilityInfo` _array_element))
    (`BlueprintMapLibrary.Map_Add` (`self.ActiveAbility`) _name (make `/Game/ExampleTimer/S_AbilityInfo` _name _description _icon _cooldown))))

(event `StartTimer`
  (params (Key :type "String (by ref)"))
  ;[0 0 0] Logic to start cooldown timer.
  (if (`BlueprintMapLibrary.Map_Contains` (`self.ActiveCooldown`) Key)
    (bind _returnvalue (`KismetSystemLibrary.K2_SetTimerDelegate` (`|CreateDelegate` :!event `TickCooldown`) 0.1 true))
    (set `self.CooldownTimerHandle` _returnvalue)))

(event `TickCooldown`
  ;[0 0 0] Logic to tick active cooldowns.
  (bind _keys (`BlueprintMapLibrary.Map_Keys` (`self.ActiveCooldown`)))
  (for _array_element _keys
    (bind _value (`BlueprintMapLibrary.Map_Find` (`self.ActiveCooldown`) _array_element))
    (if (> _value 0.0)
      (`self.OnUpdateCD` _array_element _value (`.Cooldown_8_BF185AE24CDA97F9E86730BB77BB43C4` (break `/Game/ExampleTimer/S_AbilityInfo` (`BlueprintMapLibrary.Map_Find` (`self.ActiveAbility`) _array_element))))
      (`BlueprintMapLibrary.Map_Add` (`self.ActiveCooldown`) _array_element (- _value 0.1))
      (bind _output_get (set `self.ActiveCooldown` (`self.ActiveCooldown`)))
      (if (<= (`BlueprintMapLibrary.Map_Find` _output_get _array_element) 0.0)
        (`BlueprintMapLibrary.Map_Remove` _output_get _array_element))))
  (if (<= (`BlueprintMapLibrary.Map_Length` (`self.ActiveCooldown`)) 0)
    (`KismetSystemLibrary.K2_ClearAndInvalidateTimerHandle` (`self.CooldownTimerHandle`))))

(event `Attack`
  (params (`Ability Name` :type "String (by ref)"))
  ;[0 0 0] Example Ability, to show how to apply cooldown
  (bind _cd_triggered (`self.TriggerCooldown` `Ability Name`))
  (if _cd_triggered
    (`KismetSystemLibrary.PrintString` "Attacked")))

(event `Eviscerate`
  (params (`Ability Name` :type "String (by ref)"))
  ;[0 0 0] Example Ability, to show how to apply cooldown
  (bind _cd_triggered (`self.TriggerCooldown` `Ability Name`))
  (if _cd_triggered
    (`KismetSystemLibrary.PrintString` "Eviscerated")))

(event `StunCrash`
  (params (`Ability Name` :type "String (by ref)"))
  ;[0 0 0] Example Ability, to show how to apply cooldown
  (bind _cd_triggered (`self.TriggerCooldown` `Ability Name`))
  (if _cd_triggered
    (`KismetSystemLibrary.PrintString` "Stun Crash!")))

(fn `TriggerCooldown`
  (params (AbilityName :type "String (by ref)"))
  (returns (`CD Triggered` :type Boolean))
  (bind _returnvalue (`BlueprintMapLibrary.Map_Contains` (`self.ActiveCooldown`) AbilityName))
  (if (not _returnvalue)
    (`BlueprintMapLibrary.Map_Add` (`self.ActiveCooldown`) AbilityName (`.Cooldown_8_BF185AE24CDA97F9E86730BB77BB43C4` (break `/Game/ExampleTimer/S_AbilityInfo` (`BlueprintMapLibrary.Map_Find` (`self.ActiveAbility`) AbilityName))))
    (`self.StartTimer` AbilityName)
    (return _returnvalue)))